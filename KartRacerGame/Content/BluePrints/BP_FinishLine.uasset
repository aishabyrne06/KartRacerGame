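; BP_FinishLine is a finish line actor that counts laps when a BP_Kart overlaps it.
; The kart's GetTrackProgess check decides direction: a correct crossing increments LapCount and fires OnLapProgress, while a wrong-way crossing decrements it.
; A DoOnce limits the decrement to one until the next correct crossing resets it.
; LapCount lives on this actor rather than per kart, and Tick prints it as debug output.
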(event EventBeginPlay)

(event Collision|EventActorBeginOverlap
  (params (OtherActor :type Actor%20Object%20Reference))
  ;[0.15 0.15 0.15 0.5] Cast to Kart
  (bind _asbp_kart (Utilities|Casting|CastToBP_Kart OtherActor))
  ;[0.15 0.15 0.15 0.5] If player crosses finishes the correct direction, increment and if wrong direction, decrement
  (if (Default|GetTrackProgess _asbp_kart)
    (bind _result (Math|Integer|IncrementInt (Variables|Default|GetLapCount))
      (:%20%20
        ;;[0.15 0.15 0.15 0.5] Reset value if increment
        (Default|CallOnLapProgress _result)
        (goto _label Reset)))
    (else
      (Utilities|FlowControl|DoOnce false :!label _label
        (:Completed
          (Math|Integer|DecrementInt (Variables|Default|GetLapCount)))))))

(event EventTick
  (params (DeltaSeconds :type Float%20%28single-precision%29))
  (Development|PrintString (Utilities|String|ToString(Integer) (Variables|Default|GetLapCount)) true true "(R=0.000000,G=0.660000,B=1.000000,A=1.000000)" 0.0))

(fn ConstructionScript)